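; Base tower-defense turret that tracks enemies overlapping its range, yaws toward the first and attacks on a cooldown timer that jamming can interrupt.
; Attack line-traces and branches by casting self to child classes: AoE spawns an effect actor, while Basic and Sniper deal upgrade-scaled damage plus slow.
; Sniper highest-HP targeting is only a print placeholder.
; Upgrades raise power or attach up to two distinct module components, with duplicated event and function logic.
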(event OnComponentEndOverlap(Range)
  (params (OverlappedComponent :type Primitive%20Component%20Object%20Reference) (OtherActor :type Actor%20Object%20Reference) (OtherComp :type Primitive%20Component%20Object%20Reference) (OtherBodyIndex :type Integer))
  ;[1 1 1] 사거리 벗어난 적 목표에서 제거
  (bind _asenemy_base (Utilities|Casting|CastToenemy_base OtherActor))
  (Utilities|Array|RemoveItem (Variables|Default|GetEnemyInSight) _asenemy_base))

(event Custom|PowerUpgrade
  ;[1 1 1] 출력 강화 적용
  (Variables|Default|SetPowerUp (+ (Variables|Default|GetPowerUp) (Variables|Default|GetPowerUpAmount)))
  (Variables|Default|SetPowerUpCount (+ (Variables|Default|GetPowerUpCount) 1)))

(event Custom|ModuleUpgrade
  (params (ModuleIndex :type Integer))
  (bind _modulelist (Variables|Default|GetModuleList))
  (bind _output (Utilities|Array|Get(acopy) _modulelist ModuleIndex))
  ;[1 1 1] 모듈 적용
  (if (>= (Utilities|Array|Length (Actor|GetComponentsByClass "/Game/blueprints/OnCollections/Modules/Module.Module_C")) 2)
    (Development|PrintString "Cannot Attach More Modules")
    (else
      (Utilities|IsValid (Actor|GetComponentbyClass _output)
        (:Is%20Valid
          (Development|PrintString "Cannot Attach Same Modules"))
        (:Is%20Not%20Valid
          (bind _returnvalue (Game|AddComponentbyClass _output))
          (Default|OnAdded _returnvalue)
          (Development|PrintString (Utilities|String|Append (Utilities|GetClassDisplayName _output) "Added to " (Utilities|GetClassDisplayName (Utilities|GetClass self)) "."))
          (Default|SetOwner _returnvalue self)
          (Utilities|Array|SetArrayElem (Variables|Default|GetModuleApplied) ModuleIndex true))))))

(event Custom|TowerJammed
  ;[1 1 1] 공중몹 타워 방해
  (Variables|Default|SetJammed true)
  (Variables|Default|SetJamTimer 0.0))

(event EventBeginPlay)

(event EventTick
  (params (DeltaSeconds :type Float%20%28single-precision%29))
  (for _array_element (Collision|GetOverlappingActors (Variables|Default|GetRange) "/Game/blueprints/monster/enemy_base.enemy_base_C" :!class /Script/Engine.PrimitiveComponent)
    (bind _asenemy_base (Utilities|Casting|CastToenemy_base _array_element))
    (Utilities|Array|AddUnique (Variables|Default|GetEnemyInSight) _asenemy_base))
  ;[1 1 1] 틱 이벤트 - 목표 바라보기 및 공격 타이머 계산
  (CallFunction|Lookat)
  (Variables|Default|SetAttackTimer (- (Variables|Default|GetAttackTimer) DeltaSeconds))
  (if (<= (Variables|Default|GetAttackTimer) 0.0)
    (if (Variables|Default|GetJammed)
      (Variables|Default|SetJamTimer (- (Variables|Default|GetJamTimer) DeltaSeconds))
      (if (<= (Variables|Default|GetJamTimer) 0.0)
        (Variables|Default|SetJammed false))
      (else
        (CallFunction|Attack)))))

(fn ConstructionScript)

(fn Attack
  (bind _self self)
  (bind _enemyinsight (Variables|Default|GetEnemyInSight))
  ;[1 1 1] 사거리 내 적이 있는지 확인
  (if (!= (Utilities|Array|Length _enemyinsight) 0)
    ;[1 1 1] 스나이퍼 타워 - 가장 HP 높은 적 탐색
    (Utilities|Casting|CastToSniperTower self
      (:then
        (for _array_element _enemyinsight
          (Development|PrintString "가장 높은 HP값과 해당 크리처 저장"))
        ;[1 1 1] 적중 대상이 적이 맞는지 확인
        (Collision|LineTraceByChannel (Transformation|GetWorldLocation (Variables|Default|GetShootingPoint)) (Transformation|GetWorldLocation (Variables|/Script/Engine.Actor|GetRootComponent (Variables|Default|GetTarget))) "TraceTypeQuery1" false 0 "ForDuration"))
      (:CastFailed
        (bind _outhit (Collision|LineTraceByChannel (Transformation|GetWorldLocation (Variables|Default|GetShootingPoint)) (Transformation|GetWorldLocation (Variables|/Script/Engine.Actor|GetRootComponent (Utilities|Array|Get(acopy) _enemyinsight))) "TraceTypeQuery1" false 0 "ForDuration"))))
    (bind _asenemy_base (Utilities|Casting|CastToenemy_base (.HitActor (Collision|BreakHitResult _outhit))))
    (Utilities|Casting|CastToAoETower _self
      (:then
        ;[1 1 1] AoE 타워는 이펙트 범위에서 피해 계산
        (Game|SpawnActorfromClass "/Game/blueprints/Tower/AoEEffect.AoEEffect_C" (Math|Conversions|ToTransform(Vector) (.Location (Collision|BreakHitResult _outhit))) "Undefined" 0 0)
        (Development|PrintString "AoE"))
      (:CastFailed
        (Utilities|Casting|CastToBasicTower _self
          (:then
            ;[1 1 1] 피해량 공식 = (기본 피해량 + (파워업 단계  * 파워업 수치)) * 추가 피해 비율
            (Default|TakeDamage _asenemy_base (Math|Float|Truncate (* (+ (Variables|Default|GetATK_DMG) (* (Variables|Default|GetPowerUp) (Variables|Default|GetPowerUpAmount))) (Variables|Default|GetPowerAmp))) self (.HitBoneName (Collision|BreakHitResult _outhit))))
          (:CastFailed
            (Utilities|Casting|CastToSniperTower _self)
            ;[1 1 1] 피해량 공식 = (기본 피해량 + (파워업 단계  * 파워업 수치)) * 추가 피해 비율
            (Default|TakeDamage _asenemy_base (Math|Float|Truncate (* (+ (Variables|Default|GetATK_DMG) (* (Variables|Default|GetPowerUp) (Variables|Default|GetPowerUpAmount))) (Variables|Default|GetPowerAmp))) self (.HitBoneName (Collision|BreakHitResult _outhit)))))
        (Default|AddEffect _asenemy_base (Variables|Default|GetSlowEff))))
    ;[1 1 1] 공격 타이머 리셋
    (Variables|Default|SetAttackTimer (* (Variables|Default|GetATK_SPD) (Variables|Default|GetSPD_AMP)))))

(fn Lookat
  (bind _enemyinsight (Variables|Default|GetEnemyInSight))
  (if (!= (Utilities|Array|Length _enemyinsight) 0)
    (Transformation|SetWorldRotation (Variables|Default|GetBody) (Math|Rotator|MakeRotator 0.0 0.0 (.Yaw (Math|Rotator|BreakRotator (Math|Rotator|FindLookatRotation (Transformation|GetActorLocation) (Transformation|GetActorLocation (Utilities|Array|Get(acopy) _enemyinsight)))))) false false)))

(fn ApplyModule
  (params (index :type Integer))
  (bind _modulelist (Variables|Default|GetModuleList))
  (bind _output (Utilities|Array|Get(acopy) _modulelist index))
  ;[1 1 1] 1차 필터 - 모듈이 2개 이상 적용되어 있는가?
  (if (>= (Utilities|Array|Length (Actor|GetComponentsByClass "/Game/blueprints/OnCollections/Modules/Module.Module_C")) 2)
    ;[1 1 1] 모듈 적용 불가 케이스 - return false
    (Development|PrintString "Cannot Attach More Modules")
    (else
      ;[1 1 1] 2차 필터 - 동일 종류의 모듈이 적용되어 있는가?
      (Utilities|IsValid (Actor|GetComponentbyClass _output)
        (:Is%20Valid
          (Development|PrintString "Cannot Attach Same Modules"))
        (:Is%20Not%20Valid
          ;[1 1 1] 모듈 적용 가능 케이스 - 모듈 추가 후 return true
          (bind _returnvalue (Game|AddComponentbyClass _output))
          (Default|SetOwner _returnvalue self)
          (Default|OnAdded _returnvalue)
          (Development|PrintString (Utilities|String|Append (Utilities|GetClassDisplayName _output) "Added to " (Utilities|GetClassDisplayName (Utilities|GetClass self)) "."))
          (Utilities|Array|SetArrayElem (Variables|Default|GetModuleApplied) index true)
          (return true)))))
  (return false))