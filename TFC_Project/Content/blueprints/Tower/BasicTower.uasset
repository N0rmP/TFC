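; Basic tower for a tower-defense game, a child tower class that shoots the first enemy in range.
; Construction sets its stats, Tick and LookAt defer to the parent, and range end-overlap drops departing enemies.
; Attack line-traces to the target, applies power-up-scaled damage, draws a tracer through the GameInstance's LineManager and resets the timer.
; The fourth module cumulatively raises the damage multiplier against enemies in a specific state.
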(event OnComponentEndOverlap(Range)
  (params (OverlappedComponent :type Primitive%20Component%20Object%20Reference) (OtherActor :type Actor%20Object%20Reference) (OtherComp :type Primitive%20Component%20Object%20Reference) (OtherBodyIndex :type Integer))
  ;[1 1 1] 사거리 벗어난 적 목표에서 제거
  (bind _asenemy_base (Utilities|Casting|CastToenemy_base OtherActor))
  (Utilities|Array|RemoveItem (Variables|Default|GetEnemyInSight) _asenemy_base))

(event Custom|CustomEvent_0)

(event EventTick
  (params (DeltaSeconds :type Float%20%28single-precision%29))
  (|CallParentFunction DeltaSeconds))

(fn ConstructionScript
  ;[1 1 1] 능력치 설정
  (Variables|Default|SetTowerPrice 100)
  (Variables|Default|SetATK_DMG 0)
  (Variables|Default|SetATK_SPD 1.0)
  (Variables|Default|SetATK_RANGE 2e+02)
  (Variables|Default|SetPowerUpAmount 3)
  (Development|PrintString "asdfasdfasdf"))

(fn Attack
  (bind _enemyinsight (Variables|Default|GetEnemyInSight))
  ;[1 1 1] 사거리 내 적이 있는지 확인
  (if (!= (Utilities|Array|Length _enemyinsight) 0)
    ;[1 1 1] 적중 대상이 적이 맞는지 확인
    (bind _outhit (Collision|LineTraceByChannel (Transformation|GetWorldLocation (Variables|Default|GetShootingPoint)) (Transformation|GetWorldLocation (Variables|/Script/Engine.Actor|GetRootComponent (Utilities|Array|Get(acopy) _enemyinsight))) "TraceTypeQuery1" false 0 "None"))
    (bind _asenemy_base (Utilities|Casting|CastToenemy_base (.HitActor (Collision|BreakHitResult _outhit))))
    ;[1 1 1] 4번 모듈 적용 및 대상 유효타 상태 확인
    (if (Utilities|Array|Get(acopy) (Variables|Default|GetModuleApplied) 3)
      (if (== (Variables|/Game/blueprints/monster/enemy_base.enemy_base_C|Getstate _asenemy_base) 2)
        (Variables|Default|SetPowerAmp (+ (Variables|Default|GetPowerAmp) 0.4))))
    ;[1 1 1] 피해량 공식 = (기본 피해량 + (파워업 단계  * 파워업 수치)) * 추가 피해 비율
    (Default|TakeDamage _asenemy_base (Math|Float|Truncate (* (+ (Variables|Default|GetATK_DMG) (* (Variables|Default|GetPowerUp) (Variables|Default|GetPowerUpAmount))) (Variables|Default|GetPowerAmp))) self (.HitBoneName (Collision|BreakHitResult _outhit)))
    ;[1 1 1] 탄흔 생성
    (bind _asmain_game_instance (Utilities|Casting|CastToMain_GameInstance (Game|GetGameInstance)))
    (bind _line_manager_return (Default|GetLineManager _asmain_game_instance))
    (Default|PlaceLine _line_manager_return (Transformation|GetWorldLocation (Variables|Default|GetShootingPoint)) (.Location (Collision|BreakHitResult _outhit)))
    ;[1 1 1] 공격 타이머 리셋
    (Variables|Default|SetAttackTimer (* (Variables|Default|GetATK_SPD) (Variables|Default|GetSPD_AMP)))))

(fn Lookat
  (|CallParentFunction))