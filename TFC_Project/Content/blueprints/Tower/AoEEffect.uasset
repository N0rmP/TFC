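; AoE effect actor under Tower that exists for a limited lifespan and detects the enemies it hits.
; The construction script copies Lifespan into Lifetime, which Tick counts down until the actor destroys itself.
; Collision hits on testEnemy2 actors are recorded in AlreadyHit so each enemy registers only once.
; Damage is not implemented yet; a debug print marks where the damage call belongs.
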(event OnComponentHit(Collision)
  (params (HitComponent :type Primitive%20Component%20Object%20Reference) (OtherActor :type Actor%20Object%20Reference) (OtherComp :type Primitive%20Component%20Object%20Reference) (NormalImpulse :type Vector :default "0, 0, 0") (Hit :type Hit%20Result%20Structure%20%28by%20ref%29))
  (bind _alreadyhit (Variables|Default|GetAlreadyHit))
  ;[1 1 1] 피격한 적에게 피해를 주고, 중복을 방지한다.
  (bind _astest_enemy_2 (Utilities|Casting|CastTotestEnemy2 OtherActor))
  (if (== (Utilities|Array|FindItem _alreadyhit _astest_enemy_2) -1)
    (Utilities|Array|Add _alreadyhit _astest_enemy_2)
    (Development|PrintString "Call Damage Function")))

(event EventTick
  (params (DeltaSeconds :type Float%20%28single-precision%29))
  ;[1 1 1] lifespan동안만 지속되도록 설정
  (Variables|Default|Setlifetime (- (Variables|Default|Getlifetime) DeltaSeconds))
  (if (<= (Variables|Default|Getlifetime) 0.0)
    (Development|PrintString "Hello")
    (Actor|DestroyActor)))

(fn ConstructionScript
  (Variables|Default|Setlifetime (Variables|Default|Getlifespan)))