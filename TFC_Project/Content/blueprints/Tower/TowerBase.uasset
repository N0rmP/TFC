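; TowerBase is a tower slot actor that spawns a defensive tower at its SpawnPoint.
; BuildTower maps an index to Basic, Sniper or AoE tower, stores the spawned actor and registers it with the Game Instance's TowerManager.
; BeginPlay automatically builds a Sniper tower after a one-frame delay, and an unknown index only prints an error.
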(event Custom|BuildTower
  (params (Index :type Integer))
  (bind _spawnpoint (Variables|Default|GetSpawnPoint))
  (bind _returnvalue (Transformation|GetWorldTransform _spawnpoint))
  (switch int Index
    (:Default
      (Development|PrintString "error"))
    (:0
      (bind _returnvalue_2 (Game|SpawnActorfromClass "/Game/blueprints/Tower/BasicTower.BasicTower_C" _returnvalue "Undefined" 0 0))
      (Variables|Default|SetTower _returnvalue_2)
      (bind _asmain_game_instance (Utilities|Casting|CastToMain_GameInstance (Game|GetGameInstance) :!label _label))
      (bind _tower_manager_return (Default|GetTowerManager _asmain_game_instance))
      (Default|AddTower _tower_manager_return (Variables|Default|GetTower)))
    (:1
      (bind _returnvalue_3 (Game|SpawnActorfromClass "/Game/blueprints/Tower/SniperTower.SniperTower_C" _returnvalue "Undefined" 0 0))
      (Variables|Default|SetTower _returnvalue_3)
      (goto _label))
    (:2
      (bind _returnvalue_4 (Game|SpawnActorfromClass "/Game/blueprints/Tower/AoETower.AoETower_C" _returnvalue "Undefined" 0 0))
      (Variables|Default|SetTower _returnvalue_4)
      (goto _label))))

(event EventBeginPlay
  (Class|LowEntryExtendedStandardLibrary|DelayFrames 1)
  (CallFunction|BuildTower 1))

(fn ConstructionScript)