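; Sniper tower with effectively unlimited range that hitscans its Target using damage scaled by power-up level and amplifier.
; Construction Script sets base stats; Attack line-traces to the target, damages the enemy hit and resets the attack timer.
; Modules add bonus damage against full-health enemies, aim at the "weak" socket, or apply a vulnerability effect.
; Highest-HP target search is only a print placeholder, and LookAt is empty.
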(event EventTick
  (params (DeltaSeconds :type Float%20%28single-precision%29))
  (|CallParentFunction DeltaSeconds))

(fn ConstructionScript
  ;[1 1 1] 능력치 설정
  (Variables|Default|SetTowerPrice 150)
  (Variables|Default|SetATK_DMG 100)
  (Variables|Default|SetATK_SPD 1.0)
  (Variables|Default|SetATK_RANGE 999999.0)
  (Variables|Default|SetPowerUpAmount 30))

(fn Attack
  (bind _self self)
  (bind _enemyinsight (Variables|Default|GetEnemyInSight))
  (bind _shootingpoint (Variables|Default|GetShootingPoint))
  (bind _powerupamount (Variables|Default|GetPowerUpAmount))
  (bind _atk_dmg (Variables|Default|GetATK_DMG))
  (bind _target (Variables|Default|GetTarget))
  (bind _powerup (Variables|Default|GetPowerUp))
  (bind _poweramp (Variables|Default|GetPowerAmp))
  (bind _returnvalue (Transformation|GetWorldLocation _shootingpoint))
  (bind _returnvalue_2 (* _powerup _powerupamount))
  (bind _returnvalue_3 (+ _atk_dmg _returnvalue_2))
  (bind _returnvalue_4 (* _returnvalue_3 _poweramp))
  (bind _returnvalue_5 (Math|Float|Truncate _returnvalue_4))
  (bind _returnvalue_6 (* _returnvalue_4 1.25))
  (bind _returnvalue_7 (Math|Float|Truncate _returnvalue_6))
  ;[1 1 1] 사거리 내 적이 있는지 확인
  (if (!= (Utilities|Array|Length _enemyinsight) 0)
    ;[1 1 1] 스나이퍼 타워 - 가장 HP 높은 적 탐색
    (Utilities|Casting|CastToSniperTower self)
    (for _array_element _enemyinsight
      (Development|PrintString "가장 높은 HP값과 해당 크리처 저장"))
    (if (Utilities|Array|Get(acopy) (Variables|Default|GetModuleApplied) 2)
      ;[1 1 1] 적중 대상이 적이 맞는지 확인
      (bind _outhit (Collision|LineTraceByChannel _returnvalue (Transformation|GetSocketLocation (Actor|GetComponentbyClass _target "/Script/Engine.SkeletalMeshComponent") "weak") "TraceTypeQuery1" false 0 "ForDuration"))
      (bind _asenemy_base (Utilities|Casting|CastToenemy_base (.HitActor (Collision|BreakHitResult _outhit))))
      ;[1 1 1] 모듈 1 - 최대 체력 확인
      (if (Utilities|Array|Get(acopy) (Variables|Default|GetModuleApplied))
        ;[1 1 1] 피해량 공식 = (기본 피해량 + (파워업 단계  * 파워업 수치)) * 추가 피해 비율
        (bind _max_hp_res (Default|GetMaxHp (Variables|/Game/blueprints/others/creature.creature_C|Getdamagable _asenemy_base)))
        (bind _cur_hp_res (Default|GetCurHp (Variables|/Game/blueprints/others/creature.creature_C|Getdamagable _asenemy_base)))
        (if (== _max_hp_res _cur_hp_res)
          (Default|TakeDamage _asenemy_base _returnvalue_7 _self (.HitBoneName (Collision|BreakHitResult _outhit)))
          (else
            (Default|TakeDamage _asenemy_base _returnvalue_5 _self (.HitBoneName (Collision|BreakHitResult _outhit)) :!label _label)))
        (else
          (goto _label)))
      ;[1 1 1] 모듈 4 - 플레이어가 공격 시에만 적용되는 60% 피해 증가 디버프
      (if (Utilities|Array|Get(acopy) (Variables|Default|GetModuleApplied) 3)
        (Default|AddEffect _asenemy_base "/Game/blueprints/OnCollections/Effects/Vulnerable-Effects/SniperModule4_Vul.SniperModule4_Vul_C"))
      (else
        (bind _outhit_2 (Collision|LineTraceByChannel _returnvalue (Transformation|GetWorldLocation (Variables|/Script/Engine.Actor|GetRootComponent _target)) "TraceTypeQuery1" false 0 "ForDuration"))
        (bind _asenemy_base_2 (Utilities|Casting|CastToenemy_base (.HitActor (Collision|BreakHitResult _outhit_2))))
        (if (Utilities|Array|Get(acopy) (Variables|Default|GetModuleApplied))
          (bind _max_hp_res_2 (Default|GetMaxHp (Variables|/Game/blueprints/others/creature.creature_C|Getdamagable _asenemy_base_2)))
          (bind _cur_hp_res_2 (Default|GetCurHp (Variables|/Game/blueprints/others/creature.creature_C|Getdamagable _asenemy_base_2)))
          (if (== _max_hp_res_2 _cur_hp_res_2)
            (Default|TakeDamage _asenemy_base_2 _returnvalue_7 _self (.HitBoneName (Collision|BreakHitResult _outhit_2)))
            (else
              (Default|TakeDamage _asenemy_base_2 _returnvalue_5 _self (.HitBoneName (Collision|BreakHitResult _outhit_2)) :!label _label_2)))
          (else
            (goto _label_2)))
        (if (Utilities|Array|Get(acopy) (Variables|Default|GetModuleApplied) 3)
          (Default|AddEffect _asenemy_base_2 "/Game/blueprints/OnCollections/Effects/Vulnerable-Effects/SniperModule4_Vul.SniperModule4_Vul_C"))))
    ;[1 1 1] 공격 타이머 리셋
    (Variables|Default|SetAttackTimer (* (Variables|Default|GetATK_SPD) (Variables|Default|GetSPD_AMP)))))

(fn Lookat)