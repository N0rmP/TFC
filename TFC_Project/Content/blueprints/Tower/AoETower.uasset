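; Area-of-effect tower Blueprint that extends a parent tower, setting its own price, combat stats and power-up amount in the construction script.
; Attack line-traces from the shooting point to the first enemy in sight and, on an enemy hit, spawns an AoEEffect at the impact, which handles damage.
; It then resets the attack timer from attack speed and SPDAMP.
; Enemies leaving range drop from the target list; Tick and LookAt defer to the parent.
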(event OnComponentEndOverlap(Range)
  (params (OverlappedComponent :type Primitive%20Component%20Object%20Reference) (OtherActor :type Actor%20Object%20Reference) (OtherComp :type Primitive%20Component%20Object%20Reference) (OtherBodyIndex :type Integer))
  ;[1 1 1] 사거리 벗어난 적 목표에서 제거
  (bind _asenemy_base (Utilities|Casting|CastToenemy_base OtherActor))
  (Utilities|Array|RemoveItem (Variables|Default|GetEnemyInSight) _asenemy_base))

(event EventTick
  (params (DeltaSeconds :type Float%20%28single-precision%29))
  (|CallParentFunction DeltaSeconds))

(fn ConstructionScript
  ;[1 1 1] 능력치 설정
  (Variables|Default|SetTowerPrice 200)
  (Variables|Default|SetATK_DMG 8)
  (Variables|Default|SetATK_SPD 0.2)
  (Variables|Default|SetATK_RANGE 1e+02)
  (Variables|Default|SetPowerUpAmount 3))

(fn Lookat
  (|CallParentFunction))

(fn Attack
  (bind _enemyinsight (Variables|Default|GetEnemyInSight))
  ;[1 1 1] 사거리 내 적이 있는지 확인
  (if (!= (Utilities|Array|Length _enemyinsight) 0)
    ;[1 1 1] 적중 대상이 적이 맞는지 확인
    (bind _outhit (Collision|LineTraceByChannel (Transformation|GetWorldLocation (Variables|Default|GetShootingPoint)) (Transformation|GetWorldLocation (Variables|/Script/Engine.Actor|GetRootComponent (Utilities|Array|Get(acopy) _enemyinsight))) "TraceTypeQuery1" false 0 "ForDuration"))
    (Utilities|Casting|CastToenemy_base (.HitActor (Collision|BreakHitResult _outhit)))
    ;[1 1 1] AoE 타워는 이펙트 범위에서 피해 계산
    (Game|SpawnActorfromClass "/Game/blueprints/Tower/AoEEffect.AoEEffect_C" (Math|Conversions|ToTransform(Vector) (.Location (Collision|BreakHitResult _outhit))) "Undefined" 0 0)
    ;[1 1 1] 공격 타이머 리셋
    (Variables|Default|SetAttackTimer (* (Variables|Default|GetATK_SPD) (Variables|Default|GetSPD_AMP)))))