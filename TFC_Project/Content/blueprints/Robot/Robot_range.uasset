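; Detection-range actor that tracks enemies around Robot1 and hands it a target.
; Range overlap events, plus a per-Tick overlap query, maintain the EnemyInRange list; the first enemy entering while HaveTarget is false becomes Robot.Target.
; HaveTarget clears only when the list is empty and the robot's Unfreeze is true.
; With Move set, it snaps to the robot's location inside the overlap loop, so only while enemies overlap.
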(event OnComponentBeginOverlap(Range)
  (params (OverlappedComponent :type Primitive%20Component%20Object%20Reference) (OtherActor :type Actor%20Object%20Reference) (OtherComp :type Primitive%20Component%20Object%20Reference) (OtherBodyIndex :type Integer) (bFromSweep :type Boolean) (SweepResult :type Hit%20Result%20Structure%20%28by%20ref%29))
  (bind _asenemy_base (Utilities|Casting|CastToenemy_base OtherActor))
  (Utilities|Array|AddUnique (Variables|Default|Getenemy%20in%20range) _asenemy_base)
  (if (not (Variables|Default|Gethave%20target))
    (Variables|/Game/blueprints/Robot/Robot1.Robot1_C|Settarget (Variables|Default|Getrobot) _asenemy_base)
    (Variables|Default|Sethave%20target true)))

(event OnComponentEndOverlap(Range)
  (params (OverlappedComponent :type Primitive%20Component%20Object%20Reference) (OtherActor :type Actor%20Object%20Reference) (OtherComp :type Primitive%20Component%20Object%20Reference) (OtherBodyIndex :type Integer))
  (bind _asenemy_base (Utilities|Casting|CastToenemy_base OtherActor))
  (Utilities|Array|RemoveItem (Variables|Default|Getenemy%20in%20range) _asenemy_base))

(event EventBeginPlay
  (bind _returnvalue (Actor|GetActorOfClass "/Game/blueprints/Robot/Robot1.Robot1_C"))
  (Variables|Default|Setrobot _returnvalue))

(event EventTick
  (params (DeltaSeconds :type Float%20%28single-precision%29))
  (bind _enemy_in_range (Variables|Default|Getenemy%20in%20range))
  (if (and (== (Utilities|Array|Length _enemy_in_range) 0) (Variables|/Game/blueprints/Robot/Robot1.Robot1_C|Getunfreeze (Variables|Default|Getrobot)))
    (Variables|Default|Sethave%20target false))
  (for _array_element (Collision|GetOverlappingActors (Variables|Default|GetRange) "/Game/blueprints/monster/enemy_base.enemy_base_C" :!class /Script/Engine.PrimitiveComponent)
    (bind _asenemy_base (Utilities|Casting|CastToenemy_base _array_element))
    (Utilities|Array|AddUnique _enemy_in_range _asenemy_base)
    (if (Variables|Default|Getmove)
      (Transformation|SetActorLocation (Transformation|GetActorLocation (Variables|Default|Getrobot)) false false))))

(fn ConstructionScript)