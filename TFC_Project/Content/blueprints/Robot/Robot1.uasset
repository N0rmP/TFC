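; Companion robot Blueprint that either follows the player or stands by as an area slow against enemies, depending on the Mode flag.
; BeginPlay caches the player as target; Tick drives a temporary AIMoveTo follow, guarded by a loop flag, while Mode is on.
; Otherwise it stops and applies a normal or advanced slow effect to overlapping enemies every tick, swapping the range indicator's material to show standby.
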(event Custom|move%20to
  ;[1 1 1] 이동(아직 임시)
  (if (stale _output_get)
    (bind _output_get (Variables|Default|Setloopchecker false))
    (AI|AIMoveTo self "0, 0, 0" (Variables|Default|Gettarget) 1e+01 true
      (:then
        (Variables|Default|Setloopchecker true)))))

(event EventBeginPlay
  ;[1 1 1] 초기화
  (bind _returnvalue (Actor|GetActorOfClass "/Game/blueprints/player/player_character.player_character_C"))
  (bind _output_get (Variables|Default|Setplayer _returnvalue))
  (Variables|Default|Settarget _output_get))

(event EventTick
  (params (DeltaSeconds :type Float%20%28single-precision%29))
  (bind _range_visible (Variables|Default|GetRange_Visible))
  ;[1 1 1] 대기 모드시에 범위내 enemy에게 슬로우
  (if (Variables|Default|Getmode)
    (Rendering|Material|SetMaterial _range_visible 0 "/Game/resource/temp/StarterContent/Materials/transparent.transparent")
    (CallFunction|Moveto)
    (else
      (Rendering|Material|SetMaterial _range_visible 0 "/Game/resource/material/half_transparent.half_transparent")
      (Components|Movement|StopMovementImmediately (Variables|Character|GetCharacterMovement))
      (for _array_element (Collision|GetOverlappingActors (Variables|Default|GetRange) "/Game/blueprints/monster/enemy_base.enemy_base_C" :!class /Script/Engine.PrimitiveComponent)
        (bind _asenemy_base (Utilities|Casting|CastToenemy_base _array_element))
        (if (Variables|Default|GetadvancedSlow)
          (Default|AddEffect _asenemy_base "/Game/blueprints/OnCollections/Effects/SlowEffect/AdvancedSlowEffect.AdvancedSlowEffect_C")
          (else
            (Default|AddEffect _asenemy_base "/Game/blueprints/OnCollections/Effects/SlowEffect/SlowEffect.SlowEffect_C")))))))

(fn ConstructionScript)

(fn CheckTooFar
  (params (distance :type Float%20%28single-precision%29))
  (return (>= (Math|Vector|Distance(Vector) (Transformation|GetActorLocation (Variables|Default|Getplayer)) (Transformation|GetActorLocation self)) distance)))