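; Effectable manages the effects, called OnCollections, attached to an owning creature.
; Adding one by class calls OnStacked on an existing instance of that exact class; otherwise it creates a component on the owner, tracks it in an array and calls OnAdded.
; Deleting removes it from the array and, only if it was found, calls OnDeleted and destroys the component.
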(fn SetOwner
  (params (creature_param :type Creature%20Object%20Reference))
  (Variables|Default|Setowner creature_param))

(fn AddonCollection
  (params (on_collection_class_param :type Actor%20Component%20Class%20Reference))
  (bind _on_collections (Variables|Default|Geton_collections))
  ;[1 1 1] 동일한 on_collection이 이미 존재한다면,
  ; 새롭게 추가하는 대신 기존 것의 on_stacked를 실행한다.
  (for _index (range 0 (Utilities|Array|Length _on_collections))
    (if (== (Utilities|GetClass (Utilities|Array|Get(acopy) _on_collections _index)) on_collection_class_param)
      (Default|OnStacked (Utilities|Array|Get(acopy) _on_collections _index))
      (return)))
  ;[1 1 1] 없던 on_collection이라면 add 및 on_added를 실행한다.
  (bind _returnvalue (Game|AddComponentbyClass (Variables|Default|Getowner) on_collection_class_param))
  (bind _ason_collection (Utilities|Casting|CastToOnCollection _returnvalue))
  (Utilities|Array|Add (Variables|Default|Geton_collections) _ason_collection)
  (Default|OnAdded _ason_collection))

(fn DeleteonCollection
  (params (on_collection_param :type On%20Collection%20Object%20Reference))
  (bind _returnvalue (Utilities|Array|RemoveItem (Variables|Default|Geton_collections) on_collection_param))
  (if _returnvalue
    (Default|OnDeleted on_collection_param)
    (Components|DestroyComponent on_collection_param)))