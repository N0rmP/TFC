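; Core actor whose health depends on the game's hard mode and whose death ends the level.
; On BeginPlay it reads HardMode from Main_GameInstance, sets its Damagable max HP to one in hard mode or to BaseMaxHP otherwise, then fills and prints current HP.
; The Die override calls its parent, then calls LevelEnd with false on the game instance.
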(event EventBeginPlay
  (bind _damagable (Variables|Default|Getdamagable))
  (bind _asmain_game_instance (Utilities|Casting|CastToMain_GameInstance (Game|GetGameInstance)))
  (if (Variables|/Game/blueprints/others/Observer/Main_GameInstance.Main_GameInstance_C|Gethard_mode _asmain_game_instance)
    (Default|SetMaxHp _damagable 1)
    (bind _max_hp_res (Default|GetMaxHp _damagable))
    (Default|SetCurHp _damagable _max_hp_res)
    (bind _cur_hp_res (Default|GetCurHp _damagable))
    (Development|PrintString (Utilities|String|ToString(Integer) _cur_hp_res))
    (else
      (Default|SetMaxHp _damagable (Variables|Default|Getbase_maxHP))
      (bind _max_hp_res_2 (Default|GetMaxHp _damagable))
      (Default|SetCurHp _damagable _max_hp_res_2)
      (bind _cur_hp_res_2 (Default|GetCurHp _damagable))
      (Development|PrintString (Utilities|String|ToString(Integer) _cur_hp_res_2)))))

(event Collision|EventActorBeginOverlap
  (params (OtherActor :type Actor%20Object%20Reference))
  (|CallParentFunction OtherActor) ; 지금 이 노드는 비활성 상태입니다. \n핀을 끌어서 다른 노드를 연결하면 활성화됩니다.
)

(event EventTick
  (params (DeltaSeconds :type Float%20%28single-precision%29))
  (|CallParentFunction DeltaSeconds) ; 지금 이 노드는 비활성 상태입니다. \n핀을 끌어서 다른 노드를 연결하면 활성화됩니다.
)

(fn ConstructionScript
  (|CallParentFunction))

(fn Die
  (|CallParentFunction)
  (bind _asmain_game_instance (Utilities|Casting|CastToMain_GameInstance (Game|GetGameInstance)))
  (Default|LevelEnd _asmain_game_instance false))