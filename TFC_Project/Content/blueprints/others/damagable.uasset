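; Damagable health helper that stores current and maximum HP for an owner assigned through SetOwner.
; Getters, setters and adders manage both values, calling the owner's Die whenever a result is zero or below.
; SetCurHp clamps to the valid range, but AddCurHp leaves CurHp unchanged when the sum falls outside it.
; Changing MaxHp to a positive value does not re-clamp CurHp.
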(fn GetCurHp
  (return (Variables|Default|Getcur_hp)))

(fn SetCurHp
  (params (val :type Integer))
  (LocalVariables|Settemp_hp_set val)
  (if (>= 0 (LocalVariables|Gettemp_hp_set))
    (Variables|Default|Setcur_hp 0)
    (Default|Die (Variables|Default|Getowner))
    (elif (> (LocalVariables|Gettemp_hp_set) (Variables|Default|Getmax_hp))
      (Variables|Default|Setcur_hp (Variables|Default|Getmax_hp))
      (else
        (Variables|Default|Setcur_hp (LocalVariables|Gettemp_hp_set))))))

(fn AddCurHp
  (params (val :type Integer))
  (LocalVariables|Settemp_hp_add (+ val (Variables|Default|Getcur_hp)))
  (if (>= 0 (LocalVariables|Gettemp_hp_add))
    (LocalVariables|Settemp_hp_add 0)
    (Default|Die (Variables|Default|Getowner))
    (elif (> (LocalVariables|Gettemp_hp_add) (Variables|Default|Getmax_hp))
      (LocalVariables|Settemp_hp_add (Variables|Default|Getmax_hp))
      (else
        (Variables|Default|Setcur_hp (LocalVariables|Gettemp_hp_add))))))

(fn SetOwner
  (params (val :type Creature%20Object%20Reference))
  (Variables|Default|Setowner val))

(fn GetMaxHp
  (return (Variables|Default|Getmax_hp)))

(fn AddMaxHp
  (params (val :type Integer))
  (LocalVariables|Settemp_hp_add (+ val (Variables|Default|Getmax_hp)))
  (if (>= 0 (LocalVariables|Gettemp_hp_add))
    (LocalVariables|Settemp_hp_add 0)
    (Default|Die (Variables|Default|Getowner))
    (else
      (Variables|Default|Setmax_hp (LocalVariables|Gettemp_hp_add)))))

(fn SetMaxHp
  (params (val :type Integer))
  (LocalVariables|Settemp_hp_set val)
  (if (>= 0 (LocalVariables|Gettemp_hp_set))
    (Variables|Default|Setcur_hp 0)
    (Default|Die (Variables|Default|Getowner))
    (else
      (Variables|Default|Setmax_hp (LocalVariables|Gettemp_hp_set)))))