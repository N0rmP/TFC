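; Creature is an actor Blueprint that handles damage, death and attached effects through its Damagable and Effectable members.
; The construction script sets itself as Owner of both, and AddEffect and RemoveEffect edit Effectable's OnCollections.
; TakeDamage and Die first notify every effect in that collection, then subtract HP through Damagable or destroy the actor.
; Its event graph holds only empty placeholder events, and nothing here calls Die.
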(event EventBeginPlay)

(event Collision|EventActorBeginOverlap
  (params (OtherActor :type Actor%20Object%20Reference)))

(event EventTick
  (params (DeltaSeconds :type Float%20%28single-precision%29)))

(fn ConstructionScript
  (bind _self self)
  (Variables|/Game/blueprints/others/damagable.damagable_C|Setowner (Variables|Default|Getdamagable) _self)
  (Variables|/Game/blueprints/others/effectable.effectable_C|Setowner (Variables|Default|Geteffectable) _self))

(fn Die
  (for _array_element (Variables|/Game/blueprints/others/effectable.effectable_C|Geton_collections (Variables|Default|Geteffectable))
    (Default|OnCreatureDie _array_element))
  ;[1 1 1] actual process of on_creature_dire
  (Actor|DestroyActor))

(fn TakeDamage
  (params (val :type Integer) (attacker :type Actor%20Object%20Reference) (hit_bone_name :type Name))
  (for _array_element (Variables|/Game/blueprints/others/effectable.effectable_C|Geton_collections (Variables|Default|Geteffectable))
    (Default|OnAttacked _array_element val attacker hit_bone_name))
  ;[1 1 1] actual process of on_attacked
  (Default|AddCurHp (Variables|Default|Getdamagable) (* val -1)))

(fn AddEffect
  (params (effect :type Effect%20Class%20Reference))
  (Default|AddonCollection (Variables|Default|Geteffectable) effect))

(fn RemoveEffect
  (params (effect :type Effect%20Object%20Reference))
  (Default|DeleteonCollection (Variables|Default|Geteffectable) effect))