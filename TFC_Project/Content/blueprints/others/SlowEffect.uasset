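; SlowEffect is a stackable status effect that slows its target by lowering the target's SpeedAmp.
; On_Added hands off to an existing effect of the same class via OnStacked, or registers itself and applies the initial, larger slow.
; Each stack below MaxStack deepens the slow, floored at zero, and resets Duration.
; On_Die removes one stack, restores its share of speed, and destroys the actor when none remain.
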(event EventBeginPlay
  (|CallParentFunction) ; This node is disabled and will not be called.\nDrag off pins to build functionality.
)

(event Collision|EventActorBeginOverlap
  (params (OtherActor :type Actor%20Object%20Reference))
  (|CallParentFunction OtherActor) ; This node is disabled and will not be called.\nDrag off pins to build functionality.
)

(event EventTick
  (params (DeltaSeconds :type Float%20%28single-precision%29))
  (|CallParentFunction DeltaSeconds) ; This node is disabled and will not be called.\nDrag off pins to build functionality.
)

(fn ConstructionScript
  (|CallParentFunction))

(fn OnAdded
  (params (value :type Creature%20Object%20Reference))
  (bind _output_get (Variables|Default|SetTarget value))
  (for _array_element (Variables|/Game/blueprints/others/creature.creature_C|GetEffects _output_get)
    (if (== (Utilities|GetClass self) (Utilities|GetClass _array_element))
      (CallFunction|OnStacked _array_element)
      (return)))
  (Utilities|Array|Add (Variables|/Game/blueprints/others/creature.creature_C|GetEffects _output_get) self)
  (Variables|Default|SetStack (+ (Variables|Default|GetStack) 1))
  (Variables|/Game/blueprints/others/creature.creature_C|SetSpeedAmp (Variables|Default|GetTarget) (- (Variables|/Game/blueprints/others/creature.creature_C|GetSpeedAmp (Variables|Default|GetTarget)) 0.4))
  (Variables|Default|SetDuration 4.0)
  (return))

(fn OnStacked
  (bind _target (Variables|Default|GetTarget))
  (if (not (>= (Variables|Default|GetStack) (Variables|Default|GetMaxStack)))
    (Variables|Default|SetStack (+ (Variables|Default|GetStack) 1))
    (if (>= (- (Variables|/Game/blueprints/others/creature.creature_C|GetSpeedAmp _target) 0.1) 0.0)
      (Variables|/Game/blueprints/others/creature.creature_C|SetSpeedAmp _target (- (Variables|/Game/blueprints/others/creature.creature_C|GetSpeedAmp _target) 0.1))
      (else
        (Variables|/Game/blueprints/others/creature.creature_C|SetSpeedAmp _target 0.0)))
    (Variables|Default|SetDuration 4.0)
    (return)))

(fn OnCreatureDie)

(fn OnDie
  (bind _target (Variables|Default|GetTarget))
  (if (> (Variables|Default|GetStack) 1)
    (Variables|/Game/blueprints/others/creature.creature_C|SetSpeedAmp _target (+ (Variables|/Game/blueprints/others/creature.creature_C|GetSpeedAmp _target) 0.1))
    (if (> (Variables|/Game/blueprints/others/creature.creature_C|GetSpeedAmp _target) 1.0) :!label _label
      (Variables|Default|SetSpeedAmp 1.0))
    (Variables|Default|SetStack (- (Variables|Default|GetStack) 1))
    (if (<= (Variables|Default|GetStack) 0)
      (Actor|DestroyActor :!label _label_2)
      (else
        (Development|PrintString "Done.")))
    (elif (!= (Variables|Default|GetStack) 1)
      (goto _label_2)
      (else
        (Variables|/Game/blueprints/others/creature.creature_C|SetSpeedAmp _target (+ (Variables|/Game/blueprints/others/creature.creature_C|GetSpeedAmp _target) 0.4))
        (goto _label)))))