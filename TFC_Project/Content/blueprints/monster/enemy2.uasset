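; Enemy2 is a monster child Blueprint that sets its own health and a head weak point, relying on inherited enemy logic.
; Tick uses a LoopChecker gate to run one cycle of targeting by State, short-range attack and movement, pausing briefly when the attack returns true.
; Breaking the weak point calls the parent logic, then switches State, changing the value later passed to GetTarget.
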(event EventBeginPlay
  (Variables|Default|Setindividual_max_hp 100)
  (CallFunction|EnemyInit)
  (CallFunction|GetTarget 3)
  (Variables|Default|Setstate 3)
  (Variables|Default|Setcur%20WeakPointHP 30)
  (Variables|Default|SetweakPoint "head"))

(event EventTick
  (params (DeltaSeconds :type Float%20%28single-precision%29))
  (|CallParentFunction DeltaSeconds)
  (if (Variables|Default|Getloop_checker)
    (Variables|Default|Setloop_checker false)
    (CallFunction|GetTarget (Variables|Default|Getstate))
    (bind _hit (CallFunction|EnemyAttack 50 1e+02))
    (if _hit
      (Utilities|FlowControl|Delay 1.0))
    (CallFunction|MovetoTarget)))

(fn ConstructionScript
  (|CallParentFunction))

(fn WeakPointBreak
  (|CallParentFunction)
  (Variables|Default|Setstate 2))