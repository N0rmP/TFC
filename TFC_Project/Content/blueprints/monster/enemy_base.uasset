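; Base enemy creature that chases and attacks the player, core or towers.
; GetTarget picks a target by ChaseType, MoveToTarget chases it or wanders randomly without one, and EnemyAttack deals range-checked damage.
; TakeDamage tracks weak-point bone hits toward an empty WeakPointBreak hook and calls a currently stubbed Stop on player shots.
; Die awards electricity, boosted by a tower module, and deregisters from the enemy manager; walk speed is randomized and scalable.
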(event Custom|MoveToTarget
  (bind _self self)
  (bind _target (Variables|Default|GetTarget))
  ;[1 1 1] Move_To_Target
  (if (Utilities|IsValid _target)
    (AI|AIMoveTo _self "0, 0, 0" _target 5e+01 false
      (:then
        (Variables|Default|Setloop_checker true))
      (:OnSuccess
        (if true :!label _label
          _))
      (:OnFail
        (goto _label)))
    (else
      (AI|AIMoveTo _self (+ (Transformation|GetWorldLocation (Variables|Default|GetCapsuleComponent _self)) (* (Math|Random|RandomUnitVector) 5e+02)) 0 1e+01 false
        (:OnSuccess
          _)
        (:OnFail
          _))
      (Utilities|FlowControl|Delay 0.2)
      (Variables|Default|Setloop_checker true))))

(event Custom|Stop
  (params (time :type Float%20%28single-precision%29))
  ;[1 1 1] Stop by Player Shot
)

(event EventTick
  (params (DeltaSeconds :type Float%20%28single-precision%29)))

(event EventBeginPlay
  (Variables|Default|SetWalkSpeed (* (Variables|Default|GetWalkSpeed) (Math|Random|RandomFloatinRange 1.1 1.3))))

(fn ConstructionScript
  (|CallParentFunction)
  (Variables|Default|Setcndition true)
  (bind _returnvalue (Actor|GetActorOfClass "/Game/blueprints/player/player_character.player_character_C"))
  (Variables|Default|SetTarget _returnvalue))

(fn EnemyInit
  (bind _individual_max_hp (Variables|Default|Getindividual_max_hp))
  (bind _damagable (Variables|Default|Getdamagable))
  (Default|SetMaxHp _damagable _individual_max_hp)
  (Default|SetCurHp _damagable _individual_max_hp)
  (Variables|/Game/blueprints/others/damagable.damagable_C|Setowner (Variables|Default|Getdamagable) self))

(fn GetTarget
  (params (chase%20type :type Integer))
  (bind _self self)
  (bind _returnvalue (Transformation|GetActorLocation _self))
  (switch int chase%20type
    (:1
      ;[1 1 1] Get_Target
      (Utilities|FlowControl|Sequence
        (:then_0
          (bind _outactors (Actor|GetAllActorswithTag "player")))
        (:then_1
          (bind _outactors_2 (Actor|GetAllActorswithTag "core"))
          (if (and (Utilities|IsValid (Utilities|Array|Get(acopy) _outactors)) (Utilities|IsValid (Utilities|Array|Get(acopy) _outactors_2)))
            (if (>= (Math|Vector|Distance(Vector) _returnvalue (Transformation|GetActorLocation (Utilities|Array|Get(acopy) _outactors))) (Math|Vector|Distance(Vector) (Transformation|GetActorLocation (Utilities|Array|Get(acopy) _outactors_2)) _returnvalue))
              (bind _ascreature (Utilities|Casting|CastTocreature (Utilities|Array|Get(acopy) _outactors_2)))
              (Variables|Default|SetTarget _ascreature)
              (else
                (bind _ascreature_2 (Utilities|Casting|CastTocreature (Utilities|Array|Get(acopy) _outactors)))
                (Variables|Default|SetTarget _ascreature_2)))
            (return)))))
    (:2
      (bind _outactors_3 (Actor|GetAllActorswithTag "player"))
      (if (Utilities|IsValid (Utilities|Array|Get(acopy) _outactors_3))
        (bind _ascreature_3 (Utilities|Casting|CastTocreature (Utilities|Array|Get(acopy) _outactors_3)))
        (Variables|Default|SetTarget _ascreature_3)
        (return)))
    (:3
      (bind _outactors_4 (Actor|GetAllActorswithTag "core"))
      (if (Utilities|IsValid (Utilities|Array|Get(acopy) _outactors_4))
        (bind _ascreature_4 (Utilities|Casting|CastTocreature (Utilities|Array|Get(acopy) _outactors_4)))
        (Variables|Default|SetTarget _ascreature_4)
        (return)))
    (:4
      (bind _outactors_5 (Actor|GetAllActorswithTag "player"))
      (bind _ascore (Utilities|Casting|CastTocore (Utilities|Array|Get(acopy) _outactors_5))
        (:then
          _)
        (:CastFailed
          _))
      (Variables|Default|SetTarget _ascore)
      (return))
    (:5
      (bind _outactors_6 (Actor|GetAllActorsOfClass "/Game/blueprints/Tower/Tower.Tower_C"))
      (bind (_array_element _array_index) (Utilities|Array|ForEachLoopwithBreak _outactors_6)
        (:LoopBody
          (if (== _array_index 0)
            (bind _output_get (Variables|Default|Setshortdist (Math|Vector|Distance(Vector) (Transformation|GetActorLocation self) (Transformation|GetActorLocation _array_element)) :!label _label))
            (Variables|Default|SetTarget _array_element)
            (elif (> _output_get (Math|Vector|Distance(Vector) (Transformation|GetActorLocation self) (Transformation|GetActorLocation _array_element)))
              (goto _label))))
        (:Completed
          (Utilities|Casting|CastToTower (Variables|Default|GetTarget)
            (:then
              (return))
            (:CastFailed
              (bind _outactors_7 (Actor|GetAllActorswithTag "core"))
              (if (Utilities|IsValid (Utilities|Array|Get(acopy) _outactors_7))
                (bind _ascreature_5 (Utilities|Casting|CastTocreature (Utilities|Array|Get(acopy) _outactors_7)))
                (Variables|Default|SetTarget _ascreature_5)
                (return)))))))))

(fn EnemyAttack
  (params (damage :type Integer) (range :type Float%20%28single-precision%29))
  (bind _self self)
  (bind _target (Variables|Default|GetTarget))
  (Variables|Default|SetisHit false)
  (if (Utilities|IsValid _target)
    (if (>= (Math|Vector|Distance(Vector) (Transformation|GetActorLocation _target) (Transformation|GetActorLocation _self)) range)
      (return (stale _output_get))
      (else
        (Variables|Default|SetisAttack_anim true)
        (Audio|PlaySoundatLocation (Variables|Default|Getsound_Attack) (Transformation|GetWorldLocation (Variables|Default|GetCapsuleComponent)) "0, 0, 0" 1.0 1.0 0.0 0 0 0)
        (bind _ascreature (Utilities|Casting|CastTocreature _target)
          (:then
            (CallFunction|TakeDamage _ascreature damage _self "None")
            (bind _output_get (Variables|Default|SetisHit true))
            (return _output_get))
          (:CastFailed
            (Development|PrintString "creatur_cast_fail_error")))))
    (else
      (return _output_get))))

(fn Die
  (bind _electricity_drop (Variables|Default|GetElectricity_Drop))
  (bind _lastattacker (Variables|Default|GetLastAttacker))
  (bind _asmain_game_instance (Utilities|Casting|CastToMain_GameInstance (Game|GetGameInstance)))
  (Audio|PlaySoundatLocation (Variables|Default|Getsound_Die) (Transformation|GetWorldLocation (Variables|Default|GetCapsuleComponent)) "0, 0, 0" 1.0 1.0 0.0 0 0 0)
  ;[1 1 1] 임시 추가 - 적 처치시 전력 제공
  (bind _electricity_manager_return (Default|GetElectricityManager _asmain_game_instance))
  (Utilities|IsValid _lastattacker
    (:Is%20Valid
      (bind _asbasic_tower_2 (Utilities|Casting|CastToBasicTower_2 _lastattacker)
        (:then
          (if (Utilities|Array|Get(acopy) (Variables|/Game/blueprints/Tower/Tower.Tower_C|GetModuleApplied _asbasic_tower_2) 2)
            (Default|AddElectricity _electricity_manager_return (Math|Float|Truncate (* _electricity_drop 1.2)))
            (else
              (Default|AddElectricity _electricity_manager_return _electricity_drop :!label _label))))
        (:CastFailed
          (goto _label))))
    (:Is%20Not%20Valid
      (goto _label)))
  (bind _enemy_manager_return (Default|GetEnemyManager _asmain_game_instance))
  (Default|RemoveEnemiesbyReference _enemy_manager_return self)
  (|CallParentFunction))

(fn TakeDamage
  (params (val :type Integer) (attacker :type Actor%20Object%20Reference) (hit_bone_name :type Name :default "None"))
  (|CallParentFunction val attacker "None")
  (if (not (Variables|Default|GetisBEEG))
    (bind _array_element (Utilities|Array|ForEachLoopwithBreak (Variables|Default|GetweakPoint) :!label _label)
      (:LoopBody
        (if (Utilities|Name|Equal(Name) hit_bone_name _array_element)
          (CallFunction|HitWeakPoint val)
          (Development|PrintString (Utilities|String|ToString(Name) _array_element))
          (goto _label Break)))
      (:Completed
        (bind _asplayer_character (Utilities|Casting|CastToplayer_character attacker))
        (Utilities|IsValid (Actor|GetComponentbyClass _asplayer_character "/Game/blueprints/OnCollections/Upgrades/Rifle-upgrades/Rifle_Upgrade3.Rifle_Upgrade3_C")
          (:Is%20Valid
            (CallFunction|Stop 0.3))
          (:Is%20Not%20Valid
            (CallFunction|Stop 0.2)))))))

(fn HitWeakPoint
  (params (dmg :type Integer))
  (if (not (Variables|Default|GetWP%20breaked))
    (if (>= 0 (+ (* dmg -1) (Variables|Default|Getcur%20WeakPointHP)))
      (Variables|Default|SetWP%20breaked true)
      (CallFunction|WeakPointBreak)
      (else
        (Variables|Default|Setcur%20WeakPointHP (+ (* dmg -1) (Variables|Default|Getcur%20WeakPointHP)))))))

(fn WeakPointBreak)

(fn AddSpeedAmp
  (params (SpeedAmp_param :type Float%20%28single-precision%29))
  (if (< 0.0 (+ SpeedAmp_param (stale _output_get)))
    (bind _output_get (Variables|Default|SetSpeedAmp (+ SpeedAmp_param (stale _output_get))))
    (else
      (Variables|Default|SetSpeedAmp 0.0)))
  (Variables|/Script/Engine.CharacterMovementComponent|SetMaxWalkSpeed (Variables|Character|GetCharacterMovement) (* _output_get (Variables|Default|GetWalkSpeed))))

(fn GetSpeedAmp
  (return (Variables|Default|GetSpeedAmp)))