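; Charge enemy monster Blueprint that extends a parent enemy class with its own health, weak point, electricity drop and sounds.
; Tick, gated by LoopChecker, refreshes the target for the current State, attempts a ranged-checked attack and moves toward the target.
; Breaking the weak point switches State, hides the glowing spheres and lights, and triggers a brief stun that halts walking through a Delay before restoring speed.
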(event EventBeginPlay
  (Variables|Default|Setindividual_max_hp 100)
  (CallFunction|EnemyInit)
  (CallFunction|GetTarget 3)
  (Variables|Default|Setstate 3)
  (Variables|Default|Setcur%20WeakPointHP 30)
  (Variables|Default|SetElectricity_Drop 110)
  (Variables|Default|Setsound_Attack "/Game/Assets/Small_Monster_SFX_2/Cues/Anark_Attack_01_Cue.Anark_Attack_01_Cue")
  (Variables|Default|Setsound_Die "/Game/Assets/Small_Monster_SFX_2/Cues/Anark_Death_01_Cue.Anark_Death_01_Cue"))

(event EventTick
  (params (DeltaSeconds :type Float%20%28single-precision%29))
  (|CallParentFunction DeltaSeconds)
  (if (Variables|Default|Getloop_checker)
    ;[1 1 1] Stun
    (if (== (Variables|Default|Getstun_0) 1)
      (Variables|Default|SetisStun_anim true)
      (Variables|Default|SetWalkSpeed 0.0)
      (Utilities|FlowControl|Delay 1.0)
      (Variables|Default|Setstun_0 0)
      (Variables|Default|SetWalkSpeed 4e+02)
      (Variables|Default|SetisStun_anim false))
    (Variables|Default|Setloop_checker false)
    (CallFunction|GetTarget (Variables|Default|Getstate))
    (bind _hit (CallFunction|EnemyAttack 50 2e+02))
    (if _hit
      (Utilities|FlowControl|Delay 1.0)
      (Variables|Default|SetisAttack_anim false))
    (CallFunction|MovetoTarget)))

(fn ConstructionScript
  (|CallParentFunction))

(fn WeakPointBreak
  (|CallParentFunction)
  (Variables|Default|Setstate 2)
  (Variables|Default|Setstun_0 1)
  (Rendering|Material|SetMaterial (Variables|Default|GetSphere) 0 "/Game/resource/temp/StarterContent/Materials/transparent.transparent")
  (Rendering|Components|Light|SetIntensity (Variables|Default|GetPointLight) 0.0))