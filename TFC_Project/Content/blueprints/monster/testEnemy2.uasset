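; Test monster enemy that chases and melee-attacks whichever is closer, the player or the core, both found by actor tag.
; An event loop drives it without a behavior tree: GetTarget picks the target, Attack deals delayed damage at close range, and MoveToTarget runs AIMoveTo before retargeting.
; Tick starts the loop via a Start flag, which the Stop event sets again after briefly halting movement.
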(event Custom|MoveToTarget
  (bind _self self)
  ;[1 1 1] Move_To_Target
  (AI|AIMoveTo _self "0, 0, 0" (Variables|Default|GetTarget) 5.0 true
    (:then
      (Utilities|FlowControl|Delay 1.0)
      (AI|Navigation|StopMovement (AI|GetAIController _self)))
    (:OnSuccess
      (Utilities|FlowControl|Delay 0.5))
    (:OnFail
      (Utilities|FlowControl|Delay 0.2)))
  (CallFunction|GetTarget))

(event Custom|Stop
  ;[1 1 1] Stop by Player Shot
  (Components|Movement|StopMovementImmediately (Variables|Character|GetCharacterMovement))
  (Utilities|FlowControl|Delay 0.3)
  (Variables|Default|Setstart true))

(event Custom|Attack
  (bind _self self)
  (bind _target (Variables|Default|GetTarget))
  ;[1 1 1] Attack
  (if (>= (Math|Vector|Distance(Vector) (Transformation|GetActorLocation _target) (Transformation|GetActorLocation _self)) 1e+02)
    _
    (else
      (Utilities|FlowControl|Delay 0.5)
      (Default|TakeDamage _target -10 _self "None")
      (Development|PrintString "hit!")))
  (CallFunction|MovetoTarget))

(event Custom|GetTarget
  (bind _self self)
  (bind _returnvalue (Transformation|GetActorLocation _self))
  ;[1 1 1] Get_Target
  (Utilities|FlowControl|Sequence
    (:then_0
      (bind _outactors (Actor|GetAllActorswithTag "player")))
    (:then_1
      (bind _outactors_2 (Actor|GetAllActorswithTag "core"))
      (if (and (Utilities|IsValid (Utilities|Array|Get(acopy) _outactors)) (Utilities|IsValid (Utilities|Array|Get(acopy) _outactors_2)))
        (bind _output_get (Variables|Default|Setcndition (>= (Math|Vector|Distance(Vector) _returnvalue (Transformation|GetActorLocation (Utilities|Array|Get(acopy) _outactors))) (Math|Vector|Distance(Vector) (Transformation|GetActorLocation (Utilities|Array|Get(acopy) _outactors_2)) _returnvalue))))))
    (:then_2
      (if _output_get
        (bind _ascreature (Utilities|Casting|CastTocreature (Utilities|Array|Get(acopy) _outactors_2)))
        (Variables|Default|SetTarget _ascreature)
        (else
          (bind _ascreature_2 (Utilities|Casting|CastTocreature (Utilities|Array|Get(acopy) _outactors)))
          (Variables|Default|SetTarget _ascreature_2)))
      (CallFunction|Attack))))

(event EventBeginPlay
  (bind _damagable (Variables|Default|Getdamagable))
  (Default|SetMaxHp _damagable 30)
  (Default|SetCurHp _damagable 30)
  (Variables|/Game/blueprints/others/damagable.damagable_C|Setowner (Variables|Default|Getdamagable) self))

(event EventTick
  (params (DeltaSeconds :type Float%20%28single-precision%29))
  (if (Variables|Default|Getstart)
    (CallFunction|GetTarget)
    (Variables|Default|Setstart false)))

(fn ConstructionScript
  (Actor|SetOwner self)
  (Variables|Default|Setcndition true)
  (bind _outactors (Actor|GetAllActorswithTag "player"))
  (bind _ascreature (Utilities|Casting|CastTocreature (Utilities|Array|Get(acopy) _outactors)))
  (Variables|Default|SetTarget _ascreature))