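; BEEG enemy is a heavy, high-health monster child class that starts slow-immune, chases its target and attacks it.
; Tick runs the stun and a countdown gun that fires a bullet actor when a line trace hits the player, with EnemyAttack replacing it when shooting is disabled.
; TakeDamage maps hit bones to three weakpoint pools.
; Breaking head, arm or leg removes slow immunity, gun and damage, or speed, and hides its glowing marker.
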(event Custom|CustomEvent
  (params (time :type Float%20%28single-precision%29))
  ;[1 1 1] Stop by Player Shot
  (Components|Movement|StopMovementImmediately (Variables|Character|GetCharacterMovement))
  (Utilities|FlowControl|Delay time)
  (Variables|Default|Setstart true))

(event EventBeginPlay
  ;[1 1 1] init
  (Variables|Default|SetisBEEG true)
  (Variables|Default|Setindividual_max_hp 10000)
  (CallFunction|EnemyInit)
  (CallFunction|GetTarget 1)
  (bind _output_get (Variables|Default|Setdamage 80))
  (Variables|Default|SetweakpointHP1 4000)
  (Variables|Default|SetweakpointHP2 2000)
  (Variables|Default|SetweakpointHP3 1000)
  (Variables|Default|SetElectricity_Drop 0)
  (Variables|Default|SetWalkSpeed 2e+02)
  (Variables|Default|Setguntimer 150)
  (Variables|Default|Setslow_immune true))

(event EventTick
  (params (DeltaSeconds :type Float%20%28single-precision%29))
  (bind _charactermovement (Variables|Character|GetCharacterMovement))
  (|CallParentFunction DeltaSeconds)
  (if (Variables|Default|Getloop_checker)
    (if (== (Variables|Default|Getstun_0) 1)
      (Variables|Default|SetisStun_anim true)
      (Class|NavMovementComponent|StopMovementKeepPathing _charactermovement)
      (Utilities|FlowControl|Delay 1.0)
      (Variables|Default|Setstun 0)
      (Variables|Default|SetisStun_anim false))
    (Variables|Default|Setloop_checker false)
    (CallFunction|GetTarget 2 :!label _label)
    (if (Variables|Default|Getcan_shoot)
      (if (<= (Variables|Default|Getguntimer) 0)
        (bind _shoot (CallFunction|EnemyGunReady))
        (if _shoot
          (CallFunction|EnemyGunFire (stale EventBeginPlay _output_get))
          (Variables|Default|Setguntimer 150)
          (Components|Movement|StopMovementImmediately _charactermovement)
          (Variables|Default|SetWalkSpeed 0.0)
          (Utilities|FlowControl|Delay 0.5)
          (Variables|Default|SetWalkSpeed 1.2e+02)
          (Variables|Default|SetisAttack_anim false)
          (goto _label)
          (else
            (Variables|Default|Setguntimer 20)))
        (else
          (Variables|Default|Setguntimer (- (Variables|Default|Getguntimer) 1))))
      (else
        (bind _hit (CallFunction|EnemyAttack (stale EventBeginPlay _output_get) 4e+02))
        (if _hit
          (Utilities|FlowControl|Delay 0.5)
          (Variables|Default|SetisAttack_anim false))))
    (CallFunction|MovetoTarget)))

(fn ConstructionScript
  (|CallParentFunction))

(fn WeakPointBreak
  (|CallParentFunction))

(fn TakeDamage
  (params (val :type Integer) (attacker :type Actor%20Object%20Reference) (hit_bone_name :type Name :default "None"))
  (bind _returnvalue (* val -1))
  (|CallParentFunction val attacker hit_bone_name)
  (Development|PrintString (Utilities|String|ToString(Name) hit_bone_name))
  (switch name hit_bone_name
    (:Head1
      (if (>= 0 (+ _returnvalue (Variables|Default|GetweakpointHP1)))
        (if (== (Variables|Default|GetweakpointHP1) 0)
          (Variables|Default|SetweakpointHP1 (+ _returnvalue (Variables|Default|GetweakpointHP1)) :!label _label)
          (else
            (Variables|Default|SetweakpointHP1 0)
            (CallFunction|WeakpointBreak1)
            (Development|PrintString "head beeg")))
        (else
          (goto _label))))
    (:Paw_Up_L2
      (if (>= 0 (+ _returnvalue (Variables|Default|GetweakpointHP2))) :!label _label_2
        (if (== (Variables|Default|GetweakpointHP2) 0)
          (Variables|Default|SetweakpointHP2 (+ _returnvalue (Variables|Default|GetweakpointHP2)) :!label _label_3)
          (else
            (Variables|Default|SetweakpointHP2 0)
            (CallFunction|WeakpointBreak2)
            (Development|PrintString "arm beeg")))
        (else
          (goto _label_3))))
    (:Paw_Up_L3
      (goto _label_2))
    (:Paw_F_R2
      (if (>= 0 (+ _returnvalue (Variables|Default|GetweakpointHP3))) :!label _label_4
        (if (== (Variables|Default|GetweakpointHP3) 0)
          (Variables|Default|SetweakpointHP3 (+ _returnvalue (Variables|Default|GetweakpointHP3)) :!label _label_5)
          (else
            (Variables|Default|SetweakpointHP3 0)
            (CallFunction|WeakpointBreak3)
            (Development|PrintString "legs beeg")))
        (else
          (goto _label_5))))
    (:Paw_F_R3
      (goto _label_4))
    (:Paw_F_R1
      (goto _label_4))))

(fn HitWeakpointBEEG
  (params (Dmg :type Integer) (Where :type Integer))
  (Class|LowEntryExtendedStandardLibrary|CaseSwitchInteger Where))

(fn WeakpointBreak1
  (Variables|Default|Setslow_immune false)
  (Rendering|Material|SetMaterial (Variables|Default|GetSphere) 0 "/Game/resource/temp/StarterContent/Materials/transparent.transparent")
  (Rendering|Components|Light|SetIntensity (Variables|Default|GetPointLight) 0.0))

(fn WeakpointBreak2
  (Variables|Default|Setdamage 40)
  (Variables|Default|Setcan_shoot false)
  (Variables|Default|SetisAttack_anim false)
  (Rendering|Material|SetMaterial (Variables|Default|GetSphere1) 0 "/Game/resource/temp/StarterContent/Materials/transparent.transparent")
  (Rendering|Components|Light|SetIntensity (Variables|Default|GetPointLight1) 0.0))

(fn WeakpointBreak3
  (Variables|Default|SetWalkSpeed 1.5e+02)
  (Rendering|Material|SetMaterial (Variables|Default|GetSphere2) 0 "/Game/resource/temp/StarterContent/Materials/transparent.transparent")
  (Rendering|Components|Light|SetIntensity (Variables|Default|GetPointLight2) 0.0))

(fn EnemyGunFire
  (params (damage :type Integer))
  (bind _target (Variables|Default|GetTarget))
  (bind _gun (Variables|Default|Getgun))
  (bind _gun_2 (Variables|Default|Getgun))
  (bind _returnvalue (Transformation|GetActorLocation _target))
  (bind _returnvalue_2 (Transformation|GetWorldLocation _gun_2))
  (bind _returnvalue_3 (Math|Rotator|FindLookatRotation _returnvalue_2 _returnvalue))
  (bind (_roll _pitch _yaw) (Math|Rotator|BreakRotator _returnvalue_3))
  (Variables|Default|SetisAttack_anim true)
  (Transformation|SetWorldRotation _gun (Math|Rotator|MakeRotator _roll _pitch _yaw) false false)
  (bind _returnvalue_4 (Game|SpawnActorfromClass "/Game/blueprints/monster/etc/enemy_bullet.enemy_bullet_C" (Transformation|GetWorldTransform _gun) "Undefined" 0 0))
  (Variables|/Game/blueprints/monster/etc/enemy_bullet.enemy_bullet_C|Setdamage _returnvalue_4 damage))

(fn EnemyGunReady
  (bind _outhit (Collision|LineTraceByChannel (Transformation|GetWorldLocation (Variables|Default|Getgun)) (Transformation|GetWorldLocation (Variables|/Script/Engine.Actor|GetRootComponent (Variables|Default|GetTarget))) "TraceTypeQuery1" false 0 "ForDuration"))
  (Utilities|Casting|CastToplayer_character (.HitActor (Collision|BreakHitResult _outhit))
    (:then
      (return true))
    (:CastFailed
      (return false))))