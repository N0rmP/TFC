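; Mid-size monster enemy Blueprint that sets its own health, weak point and electricity drop, then relies on inherited logic to target, attack and move.
; Tick runs a LoopChecker-gated cycle: retarget by State, attack, pause on success, then move.
; TakeDamage loops over HardPoint bones, passing half damage on a match, but full damage for every non-matching entry checked before it.
; Weak point break also clears the Cndition flag.
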(event EventBeginPlay
  (Variables|Default|Setindividual_max_hp 100)
  (CallFunction|EnemyInit)
  (CallFunction|GetTarget 3)
  (Variables|Default|Setstate 1)
  (Variables|Default|Setcur%20WeakPointHP 30)
  (Variables|Default|SetElectricity_Drop 165))

(event EventTick
  (params (DeltaSeconds :type Float%20%28single-precision%29))
  (|CallParentFunction DeltaSeconds)
  (if (Variables|Default|Getloop_checker)
    (Variables|Default|Setloop_checker false)
    (CallFunction|GetTarget (Variables|Default|Getstate))
    (bind _hit (CallFunction|EnemyAttack 50 1e+02))
    (if _hit
      (Utilities|FlowControl|Delay 1.0))
    (CallFunction|MovetoTarget)))

(fn ConstructionScript
  (|CallParentFunction))

(fn WeakPointBreak
  (|CallParentFunction)
  (Variables|Default|Setcndition false))

(fn TakeDamage
  (params (val :type Integer) (attacker :type Actor%20Object%20Reference) (hit_bone_name :type Name :default "None"))
  (bind _array_element (Utilities|Array|ForEachLoopwithBreak (Variables|Default|GethardPoint) :!label _label)
    (:LoopBody
      (if (Utilities|Name|Equal(Name) hit_bone_name _array_element)
        (|CallParentFunction (/ val 2) 0 hit_bone_name)
        (Development|PrintString "half")
        (goto _label Break)
        (else
          (|CallParentFunction val 0 hit_bone_name))))))