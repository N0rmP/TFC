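; Flying enemy that heads for its target, jams towers it finds along the way and otherwise attacks at close range.
; Tick runs a LoopChecker-gated latent loop: wait out stun, seek overlapping towers in Range, then AIMoveTo and call TowerJammed up close, or fall back to EnemyAttack and MoveToTarget.
; Breaking its weak point makes the mesh sink each tick to a set offset, pausing that loop until it lands.
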(event EventBeginPlay
  (Variables|Default|Setindividual_max_hp 30)
  (CallFunction|EnemyInit)
  (CallFunction|GetTarget 1)
  (Variables|Default|Setcur%20WeakPointHP 10)
  (Variables|Default|SetElectricity_Drop 6)
  (Variables|Default|Setdecend_value "0, 0,-97.000000"))

(event EventTick
  (params (DeltaSeconds :type Float%20%28single-precision%29))
  (bind _mesh (Variables|Character|GetMesh))
  (bind _returnvalue (Transformation|GetRelativeTransform _mesh))
  (bind _location (Math|Transform|BreakTransform _returnvalue))
  (bind _returnvalue_2 (- _location "0, 0,2.000000"))
  (|CallParentFunction DeltaSeconds)
  (if (Variables|Default|GetweakPointBreaked)
    (if (Math|Vector|NotEqual(Vector) (Variables|Default|Getdecend_value) _returnvalue_2 0.0001)
      (Transformation|SetRelativeLocation _mesh _returnvalue_2 false false)
      (else
        (if (Variables|Default|Getloop_checker) :!label _label
          (if (== (Variables|Default|Getstun) 1)
            (Utilities|FlowControl|Delay 3.0)
            (Variables|Default|Setstun 0))
          (Variables|Default|Setloop_checker false)
          (if (Variables|Default|GethaveTarget)
            ;[1 1 1] 사거리 안에 들어오면 재밍 아니면 이동
            (if (<= (Math|Vector|Distance(Vector) (Transformation|GetActorLocation self) (Transformation|GetActorLocation (stale _output_get))) 7e+01)
              (Default|TowerJammed (stale _output_get))
              (else
                (AI|AIMoveTo self "0, 0, 0" (stale _output_get) 5.0 false :!label _label_2
                  (:then
                    _)
                  (:OnSuccess
                    (Utilities|FlowControl|Delay 0.5))
                  (:OnFail
                    (Utilities|FlowControl|Delay 0.2)))))
            (Variables|Default|Setloop_checker true)
            (else
              ;[1 1 1] 코어로 직진하는 중에 범위 안에 타워 찾기
              (CallFunction|GetTarget 3)
              (for _array_element (Collision|GetOverlappingActors (Variables|Default|GetRange) "/Game/blueprints/Tower/Tower.Tower_C" :!class /Script/Engine.PrimitiveComponent)
                (bind _astower (Utilities|Casting|CastToTower _array_element))
                (bind _output_get (Variables|Default|SetTargetTower _astower))
                (Variables|Default|SethaveTarget true)
                (goto _label_2))
              (if (not (Variables|Default|GethaveTarget))
                (bind _hit (CallFunction|EnemyAttack 30 7e+01))
                (if _hit
                  (Utilities|FlowControl|Delay 0.5))
                (CallFunction|MovetoTarget)))))))
    (else
      (goto _label))))

(fn ConstructionScript
  (|CallParentFunction))

(fn WeakPointBreak
  (|CallParentFunction)
  (Variables|Default|SetweakPointBreaked true))