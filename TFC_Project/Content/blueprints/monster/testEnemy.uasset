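; Test enemy pawn that uses AI movement to head for the first actor tagged "core".
; Tick consumes a Start flag to call MoveNPC, which prints a debug string on success or failure and re-issues itself after a short delay.
; The Stop event, noted as triggered by player shots, halts movement immediately, then sets Start after a brief pause so movement resumes.
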(event Custom|MoveNPC
  (bind _outactors (Actor|GetAllActorswithTag "core"))
  (AI|AIMoveTo self (Transformation|GetActorLocation (Utilities|Array|Get(acopy) _outactors)) 0 5.0 false
    (:OnSuccess
      (Development|PrintString "Hello")
      (Utilities|FlowControl|Delay 0.5))
    (:OnFail
      (Development|PrintString "bye")
      (Utilities|FlowControl|Delay 0.2)))
  (CallFunction|MoveNPC))

(event Custom|Stop
  ;[1 1 1] Stop by Player Shot
  (Components|Movement|StopMovementImmediately (Variables|Character|GetCharacterMovement))
  (Utilities|FlowControl|Delay 0.3)
  (Variables|Default|Setstart true))

(event EventTick
  (params (DeltaSeconds :type Float%20%28single-precision%29))
  (if (Variables|Default|Getstart)
    (CallFunction|MoveNPC)
    (Variables|Default|Setstart false)))

(fn ConstructionScript)