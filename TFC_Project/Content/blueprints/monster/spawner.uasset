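; Monster spawner actor that repeatedly spawns Enemy1 AI pawns at the location of its Cube component.
; A frame-based countdown starts on BeginPlay, decrements each Tick, and resets after each spawn.
; The spawn class comes from an Enemy1 instance already found in the level, passed to SpawnEnemy.
; SpawnEnemy returns the cast pawn and a success flag, which Tick ignores.
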(event EventBeginPlay
  (Variables|Default|Settimer 200))

(event EventTick
  (params (DeltaSeconds :type Float%20%28single-precision%29))
  (if (> 0 (Variables|Default|Gettimer))
    (bind _returnvalue (Actor|GetActorOfClass "/Game/blueprints/monster/enemy1.enemy1_C"))
    (CallFunction|SpawnEnemy _returnvalue)
    (Variables|Default|Settimer 200)
    (else
      (Variables|Default|Settimer (- (Variables|Default|Gettimer) 1)))))

(fn ConstructionScript)

(fn SpawnEnemy
  (params (enemy%20type :type Creature%20Object%20Reference))
  (Variables|Default|Setsuccess true)
  (bind _returnvalue (AI|SpawnAIFromClass (Utilities|GetClass enemy%20type) 0 (Transformation|GetWorldLocation (Variables|Default|GetCube)) "0.000000, 0,0.000000" false))
  (bind _asenemy_1 (Utilities|Casting|CastToenemy1 _returnvalue)
    (:then
      _)
    (:CastFailed
      (bind _output_get (Variables|Default|Setsuccess false))))
  (return _asenemy_1 _output_get))