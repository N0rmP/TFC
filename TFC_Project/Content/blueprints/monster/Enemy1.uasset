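; Enemy1 is a monster Blueprint built on a parent enemy class, with its own HP and a breakable head weak point.
; BeginPlay initializes the enemy and acquires a target.
; Tick uses a LoopChecker gate to run a retarget, attack and move cycle, with delays for stun recovery and after successful attacks.
; Breaking the weak point calls the parent logic, deals extra damage and sets the stun.
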(event EventBeginPlay
  (Variables|Default|Setindividual_max_hp 30)
  (CallFunction|EnemyInit)
  (CallFunction|GetTarget 1)
  (Variables|Default|Setcur%20WeakPointHP 10)
  (Variables|Default|SetweakPoint "head"))

(event EventTick
  (params (DeltaSeconds :type Float%20%28single-precision%29))
  (|CallParentFunction DeltaSeconds)
  (if (Variables|Default|Getloop_checker)
    (if (== (Variables|Default|Getstun) 1)
      (Utilities|FlowControl|Delay 3.0)
      (Variables|Default|Setstun 0))
    (Variables|Default|Setloop_checker false)
    (CallFunction|GetTarget 1)
    (bind _hit (CallFunction|EnemyAttack 30 1e+02))
    (if _hit
      (Utilities|FlowControl|Delay 0.5))
    (CallFunction|MovetoTarget)))

(fn ConstructionScript
  (|CallParentFunction))

(fn WeakPointBreak
  (|CallParentFunction)
  (CallFunction|TakeDamage 10 0 "None")
  (Variables|Default|Setstun 1))