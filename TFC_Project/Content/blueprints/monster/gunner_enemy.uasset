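; Gunner monster, a child enemy that chases its target and shoots bullets at the player, with a melee fallback.
; Tick, gated by LoopChecker, counts down a frame-based gun timer, then fires only if a debug-drawn visibility trace hits the player.
; Firing snaps yaw toward the target and spawns a bullet at the gun.
; Breaking its weak point deals damage, triggers a timed stun and clears Cndition, switching it to melee attacks.
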(event EventBeginPlay
  (Variables|Default|Setindividual_max_hp 30)
  (CallFunction|EnemyInit)
  (CallFunction|GetTarget 2)
  (Variables|Default|Setcur%20WeakPointHP 10)
  (Variables|Default|SetElectricity_Drop 6)
  (Variables|Default|SetWalkSpeed 4e+02)
  (Variables|Default|Setguntimer 150))

(event EventTick
  (params (DeltaSeconds :type Float%20%28single-precision%29))
  (|CallParentFunction DeltaSeconds)
  (if (Variables|Default|Getloop_checker)
    (if (== (Variables|Default|Getstun) 1)
      (Utilities|FlowControl|Delay 3.0)
      (Variables|Default|Setstun 0))
    (Variables|Default|Setloop_checker false)
    (CallFunction|GetTarget 2 :!label _label)
    (if (Variables|Default|Getcndition)
      (if (<= (Variables|Default|Getguntimer) 0)
        (bind _shoot (CallFunction|EnemyGunReady))
        (if _shoot
          (CallFunction|EnemyGunFire)
          (Variables|Default|Setguntimer 150)
          (goto _label)
          (else
            (Variables|Default|Setguntimer 20)))
        (else
          (Variables|Default|Setguntimer (- (Variables|Default|Getguntimer) 1))))
      (else
        (bind _hit (CallFunction|EnemyAttack 30 1e+02))
        (if _hit
          (Utilities|FlowControl|Delay 0.5))))
    (CallFunction|MovetoTarget)))

(fn ConstructionScript
  (|CallParentFunction))

(fn WeakPointBreak
  (|CallParentFunction)
  (CallFunction|TakeDamage 10 0 "None")
  (Variables|Default|Setstun 1)
  (Variables|Default|Setcndition false))

(fn EnemyGunReady
  (bind _outhit (Collision|LineTraceByChannel (Transformation|GetWorldLocation (Variables|Default|GetCapsuleComponent)) (Transformation|GetWorldLocation (Variables|/Script/Engine.Actor|GetRootComponent (Variables|Default|GetTarget))) "TraceTypeQuery1" false 0 "ForDuration"))
  (Utilities|Casting|CastToplayer_character (.HitActor (Collision|BreakHitResult _outhit))
    (:then
      (return true))
    (:CastFailed
      (return false))))

(fn EnemyGunFire
  (Transformation|SetWorldRotation (Variables|Default|GetCapsuleComponent) (Math|Rotator|MakeRotator 0.0 0.0 (.Yaw (Math|Rotator|BreakRotator (Math|Rotator|FindLookatRotation (Transformation|GetActorLocation) (Transformation|GetActorLocation (Variables|Default|GetTarget)))))) false false)
  (Game|SpawnActorfromClass "/Game/blueprints/monster/etc/enemy_bullet.enemy_bullet_C" (Transformation|GetWorldTransform (Variables|Default|Getgun)) "Undefined" 0 0))