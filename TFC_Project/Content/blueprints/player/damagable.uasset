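; Player damagable Blueprint that stores current HP and exposes functions to read, set and add to it.
; SetCurHp accepts only values above zero and up to MaxHp, ignoring others instead of clamping.
; AddCurHp applies the same range check to the sum, but writes zero to CurHp when it passes, rather than the sum.
; BeginPlay and Tick are empty.
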(event EventBeginPlay)

(event EventTick
  (params (DeltaSeconds :type Float%20%28single-precision%29)))

(fn GetCurHp
  (return (Variables|Default|Getcur_hp)))

(fn SetCurHp
  (params (val :type Integer))
  (bind _output_get (LocalVariables|Settemp_hp_set val))
  (if (and (< 0 (LocalVariables|Gettemp_hp_set)) (<= (LocalVariables|Gettemp_hp_set) (Variables|Default|Getmax_hp)))
    (Variables|Default|Setcur_hp _output_get)))

(fn AddCurHp
  (params (val :type Integer))
  (LocalVariables|Settemp_hp_add (+ val (Variables|Default|Getcur_hp)))
  (if (and (< 0 (LocalVariables|Gettemp_hp_add)) (<= (LocalVariables|Gettemp_hp_add) (Variables|Default|Getmax_hp)))
    (Variables|Default|Setcur_hp 0)))