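; Player character with first-stage combat controls: movement, camera, jump, running, tool use and a toggle for the mode of the level's Robot1.
; Rifle and Terminal are child-actor tools swapped by visibility, with input forwarded to CurTool and mostly blocked while reloading or focussing.
; Damagable holds HP, which Tick regenerates after a post-hit delay; death calls LevelEnd on the game instance.
; The LevelInitiate call is unwired.
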(event EventBeginPlay
  (bind _damagable (Variables|Default|Getdamagable))
  ;[1 1 1] begin play
  (bind _returnvalue (Actor|GetActorOfClass "/Game/blueprints/Robot/Robot1.Robot1_C"))
  (Variables|Default|Setrobot _returnvalue)
  (Default|SetMaxHp _damagable (Variables|Default|Getplr_max_hp))
  (bind _max_hp_res (Default|GetMaxHp _damagable))
  (Default|SetCurHp _damagable _max_hp_res))

(event EventTick
  (params (DeltaSeconds :type Float%20%28single-precision%29))
  ;[1 1 1] tick
  (CallFunction|HpGenerate DeltaSeconds))

(event Input|ActionEvents|InputActionaction_input_left_click
  (params (Key :type Key%20Structure :default "None"))
  (bind _is_reloading (Variables|Default|Getis_reloading))
  (bind _cur_tool (Variables|Default|Getcur_tool))
  (bind _is_focussing (Variables|Default|Getis_focussing))
  (bind _returnvalue (or _is_reloading _is_focussing))
  ;[1 1 1] tool use
  (:Pressed
    (if (not _returnvalue)
      (Default|LeftClickon _cur_tool)))
  (:Released
    (if (not _returnvalue)
      (Default|LeftClickOff _cur_tool))))

(event Input|ActionEvents|InputActionaction_input_right_click
  (params (Key :type Key%20Structure :default "None"))
  (bind _cur_tool (Variables|Default|Getcur_tool))
  (bind _is_reloading (Variables|Default|Getis_reloading))
  (bind _is_focussing (Variables|Default|Getis_focussing))
  (bind _returnvalue (or _is_reloading _is_focussing))
  ;[1 1 1] tool use
  (:Pressed
    (if (not _returnvalue)
      (Default|RightClickon _cur_tool)))
  (:Released
    (if (not _returnvalue)
      (Default|RightClickOff _cur_tool))))

(event Input|ActionEvents|InputActionaction_input_R
  (params (Key :type Key%20Structure :default "None"))
  ;[1 1 1] tool use
  (:Pressed
    (if (not (or (Variables|Default|Getis_reloading) (Variables|Default|Getis_focussing)))
      (Default|RButton (Variables|Default|Getcur_tool)))))

(event Input|ActionEvents|InputActionaction_input_robot
  (params (Key :type Key%20Structure :default "None"))
  (bind _robot (Variables|Default|Getrobot))
  ;[1 1 1] 로봇 모드 전환
  (:Pressed
    (if (Variables|/Game/blueprints/Robot/Robot1.Robot1_C|Getmode _robot)
      (Variables|/Game/blueprints/Robot/Robot1.Robot1_C|Setmode _robot false)
      (else
        (Variables|/Game/blueprints/Robot/Robot1.Robot1_C|Setmode _robot true)))))

(event Input|ActionEvents|InputActionaction_input_1
  (params (Key :type Key%20Structure :default "None"))
  ;[1 1 1] tool use
  (:Pressed
    (if (not (or (Variables|Default|Getis_reloading) (Variables|Default|Getis_focussing)))
      (CallFunction|SwapTool))))

(event Input|ActionEvents|InputActionaction_input_2
  (params (Key :type Key%20Structure :default "None"))
  ;[1 1 1] tool use
  (:Pressed
    (if (not (or (Variables|Default|Getis_reloading) (Variables|Default|Getis_focussing)))
      (CallFunction|SwapTool 1))))

(event Input|AxisEvents|InputAxisaxis_input_mouse_wheel
  (params (AxisValue :type Float%20%28single-precision%29))
  (bind _returnvalue (Math|Float|Truncate AxisValue))
  (bind _cur_tool_index (Variables|Default|Getcur_tool_index))
  (bind _returnvalue_2 (+ _returnvalue _cur_tool_index))
  (bind _returnvalue_3 (Math|Integer|Clamp(Integer) _returnvalue_2 0 1))
  ;[1 1 1] tool use
  (if (not (and (or (Variables|Default|Getis_reloading) (Variables|Default|Getis_focussing)) (== (Variables|Default|Getcur_tool_index) _returnvalue_3)))
    (CallFunction|SwapTool _returnvalue_3)))

(event Input|AxisEvents|InputAxisaxis_input_mouse_x
  (params (AxisValue :type Float%20%28single-precision%29))
  ;[1 1 1] camera
  (if (not (Variables|Default|Getis_focussing))
    (Pawn|Input|AddControllerYawInput AxisValue)))

(event Input|AxisEvents|InputAxisaxis_input_mouse_y
  (params (AxisValue :type Float%20%28single-precision%29))
  ;[1 1 1] camera
  (if (not (Variables|Default|Getis_focussing))
    (Transformation|AddLocalRotation (Variables|Default|Getcamera_arm) (Math|Rotator|MakeRotator 0.0 (* -2 AxisValue) 0.0) false false)))

(event Input|AxisEvents|InputAxisaxis_input_forward_backward
  (params (AxisValue :type Float%20%28single-precision%29))
  (bind _returnvalue (Transformation|GetActorForwardVector))
  ;[1 1 1] movement
  (Pawn|Input|AddMovementInput (Math|Vector|Normalize (Math|Vector|MakeVector (.x _returnvalue) (.y _returnvalue) 0.0)) AxisValue false)
  (CallFunction|SetIsDash (> (* AxisValue (stale Input|AxisEvents|InputAxisaxis_input_dash AxisValue)) 0.0)))

(event Input|AxisEvents|InputAxisaxis_input_dash
  (params (AxisValue :type Float%20%28single-precision%29))
  ;[1 1 1] movement
  (if (> (* (stale Input|AxisEvents|InputAxisaxis_input_forward_backward AxisValue) AxisValue) 0.0)
    (Variables|/Script/Engine.CharacterMovementComponent|SetMaxWalkSpeed (Variables|Character|GetCharacterMovement) (Variables|Default|Getrun_speed))
    (else
      (Variables|/Script/Engine.CharacterMovementComponent|SetMaxWalkSpeed (Variables|Character|GetCharacterMovement) (Variables|Default|Getwalk_speed)))))

(event Input|AxisEvents|InputAxisaxis_input_left_right
  (params (AxisValue :type Float%20%28single-precision%29))
  ;[1 1 1] movement
  (Pawn|Input|AddMovementInput (Transformation|GetActorRightVector) AxisValue false))

(event Input|AxisEvents|InputAxisaxis_input_jump
  (params (AxisValue :type Float%20%28single-precision%29))
  ;[1 1 1] movement
  (if (> AxisValue 0.0)
    (Character|Jump)))

(fn ConstructionScript
  (bind _rifle (Variables|Default|Getrifle))
  (|CallParentFunction)
  (Utilities|Array|Add (Variables|Default|Gettool_list) _rifle)
  (Utilities|Array|Add (Variables|Default|Gettool_list) (Variables|Default|Getterminal))
  (for _array_element (Variables|Default|Gettool_list)
    (Rendering|SetVisibility _array_element false false)
    (bind _asabst_tool (Utilities|Casting|CastToabst_tool (Variables|/Script/Engine.ChildActorComponent|GetChildActor _array_element))
      (:then
        (Variables|/Game/blueprints/player/tool/abst_tool.abst_tool_C|Settool_owner _asabst_tool self))
      (:CastFailed
        (Development|PrintString "Hello"))))
  (Rendering|SetVisibility _rifle true false)
  (bind _asabst_tool_2 (Utilities|Casting|CastToabst_tool (Variables|/Script/Engine.ChildActorComponent|GetChildActor _rifle)))
  (Variables|Default|Setcur_tool _asabst_tool_2)
  (Variables|Default|Setcur_tool_index 0))

(fn GetIsDash
  (return (Variables|Default|Getis_dash)))

(fn SetIsDash
  (params (val :type Boolean))
  (Variables|Default|Setis_dash val)
  (return))

(fn GetIsFocussing
  (return (Variables|Default|Getis_focussing)))

(fn SetIsFocussing
  (params (val :type Boolean))
  (Variables|Default|Setis_focussing val))

(fn GetIsReloading
  (return (Variables|Default|Getis_reloading)))

(fn SetIsReloading
  (params (val :type Boolean))
  (Variables|Default|Setis_reloading val))

(fn GetLinetracing
  (bind _normal_camera (Variables|Default|Getnormal_camera))
  (bind _returnvalue (Transformation|GetWorldLocation _normal_camera))
  (bind _outhit (Collision|LineTraceByChannel _returnvalue (+ _returnvalue (* (Math|Vector|GetForwardVector (Transformation|GetWorldRotation _normal_camera)) 2e+03)) "TraceTypeQuery1" false 0 "None"))
  (return _outhit))

(fn SetZoom
  (params (zoom_FOV_angle :type Float%20%28single-precision%29))
  (Camera|SetFieldOfView (Variables|Default|Getnormal_camera) zoom_FOV_angle))

(fn SwapTool
  (params (tool_index :type Integer))
  (bind _tool_list (Variables|Default|Gettool_list))
  (bind _output (Utilities|Array|Get(acopy) _tool_list tool_index))
  (Rendering|SetVisibility (Utilities|Array|Get(acopy) (Variables|Default|Gettool_list) (Variables|Default|Getcur_tool_index)) false false)
  (bind _asabst_tool (Utilities|Casting|CastToabst_tool (Variables|/Script/Engine.ChildActorComponent|GetChildActor _output)))
  (Variables|Default|Setcur_tool _asabst_tool)
  (Variables|Default|Setcur_tool_index tool_index)
  (Rendering|SetVisibility _output true false))

(fn HpGenerate
  (params (val :type Float%20%28single-precision%29))
  (bind _damagable (Variables|Default|Getdamagable))
  (if (<= (Variables|Default|Gethp_gen_cur_timer) 0.0)
    (bind _cur_hp_res (Default|GetCurHp _damagable))
    (bind _max_hp_res (Default|GetMaxHp _damagable))
    (if (not (== _cur_hp_res _max_hp_res))
      (Default|AddCurHp _damagable (Variables|Default|Gethp_gen_amount))
      (Variables|Default|Sethp_gen_cur_timer 1.0)
      (bind _cur_hp_res_2 (Default|GetCurHp (Variables|Default|Getdamagable)))
      (Development|PrintString (Utilities|String|Append "after hp generate : " (Utilities|String|ToString(Integer) _cur_hp_res_2))))
    (else
      (Variables|Default|Sethp_gen_cur_timer (- (Variables|Default|Gethp_gen_cur_timer) val)))))

(fn TakeDamage
  (params (val :type Integer) (attacker :type Actor%20Object%20Reference) (hit_bone_name :type Name :default "None"))
  (|CallParentFunction val attacker hit_bone_name)
  (bind _cur_hp_res (Default|GetCurHp (Variables|Default|Getdamagable)))
  (if (> _cur_hp_res 0)
    (Variables|Default|Sethp_gen_cur_timer (Variables|Default|Gethp_gen_max_timer))
    (else
      (bind _asmain_game_instance (Utilities|Casting|CastToMain_GameInstance (Game|GetGameInstance)))
      (Default|LevelEnd _asmain_game_instance false))))