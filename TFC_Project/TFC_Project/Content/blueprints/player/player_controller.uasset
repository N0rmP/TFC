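; Player controller Blueprint that handles mouse look and directional movement for the controlled pawn.
; Mouse axes feed yaw and pitch input, while movement axes add input along the control rotation's forward and right vectors.
; Forward movement uses the full control rotation, pitch included, and its event prints that forward vector as debug output.
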(event Input|AxisEvents|InputAxismouse_y
  (params (AxisValue :type Float%20%28single-precision%29))
  (Class|PlayerController|AddPitchInput AxisValue))

(event Input|AxisEvents|InputAxismouse_x
  (params (AxisValue :type Float%20%28single-precision%29))
  (Class|PlayerController|AddYawInput AxisValue))

(event Input|AxisEvents|InputAxisforward_backward
  (params (AxisValue :type Float%20%28single-precision%29))
  (bind _returnvalue (Pawn|GetControlRotation :!class /Script/Engine.Controller))
  (bind _returnvalue_2 (Math|Vector|GetForwardVector _returnvalue))
  (Pawn|Input|AddMovementInput (Pawn|GetControlledPawn) _returnvalue_2 AxisValue false)
  (Development|PrintString (Utilities|String|ToString(Vector) _returnvalue_2)))

(event Input|AxisEvents|InputAxisleft_right
  (params (AxisValue :type Float%20%28single-precision%29))
  (Pawn|Input|AddMovementInput (Pawn|GetControlledPawn) (Math|Vector|GetRightVector (Pawn|GetControlRotation :!class /Script/Engine.Controller)) AxisValue false))

(fn ConstructionScript)